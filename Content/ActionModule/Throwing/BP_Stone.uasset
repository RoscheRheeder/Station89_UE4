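; Throwable stone actor that flies as a physics object and makes visualized noise when it bounces.
; Collision and physics stay off until Throw enables them and sets the launch velocity.
; Hit prints speed and, above a threshold, spawns a bounce sound and a sound bubble.
; A DoOnce throttles hits, resetting after a short delay only on that successful path; older MakeNoise logic is disconnected.
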(event OnComponentHit(ObjectMesh)
  (params (HitComponent :type Primitive%20Component%20Object%20Reference) (OtherActor :type Actor%20Object%20Reference) (OtherComp :type Primitive%20Component%20Object%20Reference) (NormalImpulse :type Vector :default "0, 0, 0") (Hit :type Hit%20Result%20Structure%20%28by%20ref%29))
  ;[1 1 1] Rock noise on collision
)

(event EventBeginPlay
  (bind _objectmesh (Variables|Default|GetObjectMesh))
  ;[1 1 1] Ensure collision and physics are enabled
  (Collision|SetCollisionEnabled _objectmesh "NoCollision")
  (Physics|SetSimulatePhysics _objectmesh false))

(event EventThrow
  (params (LaunchVelocity :type Vector :default "0, 0, 0"))
  (bind _objectmesh (Variables|Default|GetObjectMesh))
  ;[1 1 1] Force added to throw rock
  (Collision|SetCollisionEnabled _objectmesh "QueryAndPhysics")
  (Physics|SetSimulatePhysics _objectmesh true)
  (Class|PrimitiveComponent|SetAllPhysicsLinearVelocity _objectmesh LaunchVelocity false))

(event Collision|EventHit
  (params (MyComp :type Primitive%20Component%20Object%20Reference) (Other :type Actor%20Object%20Reference) (OtherComp :type Primitive%20Component%20Object%20Reference) (bSelfMoved :type Boolean) (HitLocation :type Vector :default "0, 0, 0") (HitNormal :type Vector :default "0, 0, 0") (NormalImpulse :type Vector :default "0, 0, 0") (Hit :type Hit%20Result%20Structure%20%28by%20ref%29))
  ;[1 1 1] Rock noise on collision with sound visualization.
  (Utilities|FlowControl|DoOnce false :!label _label
    (:Completed
      (bind _velocity (CallFunction|GetComponentVelocity MyComp "NewEnumerator0"))
      (Development|PrintString (Utilities|String|Append "Stone Velocity: " (Utilities|String|ToString(Float) _velocity)))
      (if (> _velocity 25.0)
        (Audio|SpawnSoundatLocation "/Game/ActionModule/Throwing/SC_StoneBounceCue.SC_StoneBounceCue" HitLocation "0, 0, 0" 1.0 1.0 0.0 0 0)
        (Utilities|Casting|CastToThirdPersonGameMode (Game|GetGameMode))
        (CallFunction|SpawnSoundBubbleatActor MyComp 0.5)
        (Utilities|FlowControl|Delay 0.2)
        (goto _label Reset)))))

(fn ConstructionScript)

(fn IsThrowable
  (return true))