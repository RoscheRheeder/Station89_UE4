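; BP_HRFunctions is a general-purpose function library for actor lookup, value negation and unit-aware velocity, distance and location math.
; It finds actors by class or index and recursively gathers all attached actors.
; Unit-based getters and setters match the chosen unit in a Unit array and scale by the parallel Value entry.
; Converters select a factor array by source unit and index it by target unit, forming a lookup matrix.
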(fn GetAllAttachedActorsInternal
  (params (RootActor :type Actor%20Object%20Reference) (Result :type Array%20of%20Actor%20Object%20References))
  (for _array_element (Actor|GetAttachedActors RootActor true)
    (Utilities|FlowControl|Sequence
      (:then_0
        (Utilities|Array|Add Result _array_element))
      (:then_1
        (AllAttachedActors|GetAllAttachedActorsInternal _array_element Result)))))

(fn GetAllAttachedActors
  (params (RootActor :type Actor%20Object%20Reference))
  (bind _result (LocalVariables|GetResult))
  (AllAttachedActors|GetAllAttachedActorsInternal RootActor _result)
  (return _result))

(fn GetActorOfClass
  (params (Actor%20Class :type Actor%20Class%20Reference))
  (bind _outactors (Actor|GetAllActorsOfClass 0 Actor%20Class))
  (return (Utilities|Array|Get(acopy) _outactors)))

(fn GetActorOfClassbySelectedIndex
  (params (ActorClass :type Actor%20Class%20Reference) (Index :type Integer))
  (bind _outactors (Actor|GetAllActorsOfClass 0 ActorClass))
  (return (Utilities|Array|Get(acopy) _outactors Index)))

(fn GetActorVelocity
  (params (Actor :type Actor%20Object%20Reference) (Velocity%20Unit :type Enum_Velocity%20Enum :default "NewEnumerator0"))
  (for (_array_element _array_index) (LocalVariables|GetUnit)
    (if (== _array_element Velocity%20Unit)
      (return (* (Utilities|Array|Get(acopy) (LocalVariables|GetValue) _array_index) (Math|Vector|VectorLength (Transformation|GetVelocity Actor))) Velocity%20Unit))))

(fn GetActorVelocity(Int)
  (params (Actor :type Actor%20Object%20Reference) (Velocity%20Unit :type Enum_Velocity%20Enum :default "NewEnumerator0"))
  (for (_array_element _array_index) (LocalVariables|GetUnit)
    (if (== _array_element Velocity%20Unit)
      (return (Math|Float|Truncate (* (Utilities|Array|Get(acopy) (LocalVariables|GetValue) _array_index) (Math|Vector|VectorLength (Transformation|GetVelocity Actor)))) Velocity%20Unit))))

(fn GetComponentVelocity
  (params (Component :type Scene%20Component%20Object%20Reference) (Velocity%20Unit :type Enum_Velocity%20Enum :default "NewEnumerator0"))
  (for (_array_element _array_index) (LocalVariables|GetUnit)
    (if (== _array_element Velocity%20Unit)
      (return (* (Utilities|Array|Get(acopy) (LocalVariables|GetValue) _array_index) (Math|Vector|VectorLength (Transformation|GetComponentVelocity Component))) Velocity%20Unit))))

(fn GetComponentVelocity(Int)
  (params (Component :type Scene%20Component%20Object%20Reference) (Velocity%20Unit :type Enum_Velocity%20Enum :default "NewEnumerator0"))
  (for (_array_element _array_index) (LocalVariables|GetUnit)
    (if (== _array_element Velocity%20Unit)
      (return (Math|Float|Truncate (* (Utilities|Array|Get(acopy) (LocalVariables|GetValue) _array_index) (Math|Vector|VectorLength (Transformation|GetComponentVelocity Component)))) Velocity%20Unit))))

(fn ReverseValue(Boolean)
  (params (Value :type Boolean))
  (return (Math|Conversions|ToBoolean(Integer) (Utilities|Select :Index (Math|Conversions|ToInteger(Boolean) Value) :Option%200 1 :Option%201 0))))

(fn ReverseValue(Float)
  (params (Value :type Float%20%28single-precision%29))
  (return (* Value -1.0)))

(fn ReverseValue(Integer)
  (params (Value :type Integer))
  (return (* Value -1)))

(fn ReverseValue(Integer64)
  (params (Value :type Integer64))
  (return (* Value -1)))

(fn ReverseValue(Rotator)
  (params (Value :type Rotator))
  (return (* Value -1)))

(fn ReverseValue(Vector)
  (params (Value :type Vector))
  (return (* Value -1)))

(fn ReverseValue(LinearColor)
  (params (Value :type Linear%20Color%20Structure))
  (return (* Value -1.0)))

(fn GetDistance(Vector)
  (params (A :type Vector) (B :type Vector) (Distance%20Unit :type Enum_Distance%20Enum :default "NewEnumerator0"))
  (bind _output_get (LocalVariables|SetLocation_A A))
  (bind _output_get_2 (LocalVariables|SetLocation_B B))
  (for (_array_element _array_index) (LocalVariables|GetUnit)
    (if (== _array_element Distance%20Unit)
      (return (* (Utilities|Array|Get(acopy) (LocalVariables|GetValue) _array_index) (Math|Float|Sqrt (+ (Math|Float|Square (- (.x _output_get_2) (.x _output_get))) (Math|Float|Square (- (.y _output_get_2) (.y _output_get))) (Math|Float|Square (- (.z _output_get_2) (.z _output_get)))))) Distance%20Unit))))

(fn GetDistanceBetweenActors
  (params (Actor%20A :type Actor%20Object%20Reference) (Actor%20B :type Actor%20Object%20Reference) (Distance%20Unit :type Enum_Distance%20Enum :default "NewEnumerator0"))
  (bind _output_get (LocalVariables|SetLocation_A (Transformation|GetActorLocation Actor%20A)))
  (bind _output_get_2 (LocalVariables|SetLocation_B (Transformation|GetActorLocation Actor%20B)))
  (for (_array_element _array_index) (LocalVariables|GetUnit)
    (if (== _array_element Distance%20Unit)
      (return (* (Utilities|Array|Get(acopy) (LocalVariables|GetValue) _array_index) (Math|Float|Sqrt (+ (Math|Float|Square (- (.x _output_get_2) (.x _output_get))) (Math|Float|Square (- (.y _output_get_2) (.y _output_get))) (Math|Float|Square (- (.z _output_get_2) (.z _output_get)))))) Distance%20Unit))))

(fn GetDistanceBetweenComponents
  (params (Component%20A :type Scene%20Component%20Object%20Reference) (Component%20B :type Scene%20Component%20Object%20Reference) (Distance%20Unit :type Enum_Distance%20Enum :default "NewEnumerator0"))
  (bind _output_get (LocalVariables|SetLocation_A (Transformation|GetWorldLocation Component%20A)))
  (bind _output_get_2 (LocalVariables|SetLocation_B (Transformation|GetWorldLocation Component%20B)))
  (for (_array_element _array_index) (LocalVariables|GetUnit)
    (if (== _array_element Distance%20Unit)
      (return (* (Utilities|Array|Get(acopy) (LocalVariables|GetValue) _array_index) (Math|Float|Sqrt (+ (Math|Float|Square (- (.x _output_get_2) (.x _output_get))) (Math|Float|Square (- (.y _output_get_2) (.y _output_get))) (Math|Float|Square (- (.z _output_get_2) (.z _output_get)))))) Distance%20Unit))))

(fn SetActorLocationbyUnit
  (params (Target :type Actor%20Object%20Reference) (LocationUnit :type Enum_Distance%20Enum :default "NewEnumerator0") (NewLocation :type Vector) (bSweep :type Boolean) (bTeleport :type Boolean))
  (for (_array_element _array_index) (LocalVariables|GetUnit)
    (if (== _array_element LocationUnit)
      (bind (_sweephitresult _returnvalue) (Transformation|SetActorLocation Target (* NewLocation (Utilities|Array|Get(acopy) (LocalVariables|GetValue) _array_index)) bSweep bTeleport))
      (return _sweephitresult _returnvalue LocationUnit))))

(fn SetWorldLocationbyUnit
  (params (Target :type Scene%20Component%20Object%20Reference) (LocationUnit :type Enum_Distance%20Enum :default "NewEnumerator0") (NewLocation :type Vector) (bSweep :type Boolean) (bTeleport :type Boolean))
  (for (_array_element _array_index) (LocalVariables|GetUnit)
    (if (== _array_element LocationUnit)
      (bind _sweephitresult (Transformation|SetWorldLocation Target (* NewLocation (Utilities|Array|Get(acopy) (LocalVariables|GetValue) _array_index)) bSweep bTeleport))
      (return _sweephitresult LocationUnit))))

(fn SetPhysicsLinearVelocitybyUnit
  (params (Target :type Primitive%20Component%20Object%20Reference) (VelocityUnit :type Enum_Velocity%20Enum :default "NewEnumerator0") (Converted :type Boolean) (NewVel :type Vector) (bAddToCurrent :type Boolean) (BoneName :type Name :default "None"))
  (if Converted
    (Physics|SetPhysicsLinearVelocity Target NewVel bAddToCurrent BoneName)
    (return)
    (else
      (bind (_array_element _array_index) (Utilities|Array|ForEachLoopwithBreak (LocalVariables|GetUnit) :!label _label)
        (:LoopBody
          (if (== _array_element VelocityUnit)
            (goto _label Break)))
        (:Completed
          (Physics|SetPhysicsLinearVelocity Target (* NewVel (Utilities|Array|Get(acopy) (LocalVariables|GetValue) _array_index)) bAddToCurrent "None")
          (return))))))

(fn ConvertVelocitybyUnit
  (params (CurrentVelocityUnit :type Enum_Velocity%20Enum :default "NewEnumerator0") (NewVelocityUnit :type Enum_Velocity%20Enum :default "NewEnumerator0") (Velocity :type Float%20%28single-precision%29))
  (bind (_array_element _array_index) (Utilities|Array|ForEachLoopwithBreak (LocalVariables|GetUnit) :!label _label)
    (:LoopBody
      (if (== _array_element CurrentVelocityUnit)
        (goto _label Break)))
    (:Completed
      (for (_array_element_2 _array_index_2) (LocalVariables|GetUnit)
        (if (== _array_element_2 NewVelocityUnit)
          (LocalVariables|SetSelectedUnits (Utilities|Array|MakeArray _array_index _array_index_2))
          (LocalVariables|SetNewCurrentUnit _array_element_2)))
      (return (* (Utilities|Array|Get(acopy) (Utilities|Select :Index (Utilities|Array|Get(acopy) (LocalVariables|GetSelectedUnits)) :Option%200 (LocalVariables|GetCm/s) :Option%201 (LocalVariables|GetM/s) :Option%202 (LocalVariables|GetKm/h) :Option%203 (LocalVariables|Getft/s) :Option%204 (LocalVariables|GetKnots) :Option%205 (LocalVariables|GetMph)) (Utilities|Array|Get(acopy) (LocalVariables|GetSelectedUnits) 1)) Velocity) (LocalVariables|GetNewCurrentUnit)))))

(fn ConvertVelocitybyUnit(Int)
  (params (CurrentVelocityUnit :type Enum_Velocity%20Enum :default "NewEnumerator0") (NewVelocityUnit :type Enum_Velocity%20Enum :default "NewEnumerator0") (Velocity :type Integer))
  (bind (_array_element _array_index) (Utilities|Array|ForEachLoopwithBreak (LocalVariables|GetUnit) :!label _label)
    (:LoopBody
      (if (== _array_element CurrentVelocityUnit)
        (goto _label Break)))
    (:Completed
      (for (_array_element_2 _array_index_2) (LocalVariables|GetUnit)
        (if (== _array_element_2 NewVelocityUnit)
          (LocalVariables|SetSelectedUnits (Utilities|Array|MakeArray _array_index _array_index_2))
          (LocalVariables|SetNewCurrentUnit _array_element_2)))
      (return (Math|Float|Truncate (* (Utilities|Array|Get(acopy) (Utilities|Select :Index (Utilities|Array|Get(acopy) (LocalVariables|GetSelectedUnits)) :Option%200 (LocalVariables|GetCm/s) :Option%201 (LocalVariables|GetM/s) :Option%202 (LocalVariables|GetKm/h) :Option%203 (LocalVariables|Getft/s) :Option%204 (LocalVariables|GetKnots) :Option%205 (LocalVariables|GetMph)) (Utilities|Array|Get(acopy) (LocalVariables|GetSelectedUnits) 1)) (Math|Conversions|ToFloat(Integer) Velocity))) (LocalVariables|GetNewCurrentUnit)))))

(fn ConvertDistancebyUnit
  (params (CurrentDistanceUnit :type Enum_Distance%20Enum :default "NewEnumerator0") (NewDistanceUnit :type Enum_Distance%20Enum :default "NewEnumerator0") (Distance :type Float%20%28single-precision%29))
  (bind (_array_element _array_index) (Utilities|Array|ForEachLoopwithBreak (LocalVariables|GetUnit) :!label _label)
    (:LoopBody
      (if (== _array_element CurrentDistanceUnit)
        (goto _label Break)))
    (:Completed
      (for (_array_element_2 _array_index_2) (LocalVariables|GetUnit)
        (if (== _array_element_2 NewDistanceUnit)
          (LocalVariables|SetSelectedUnits (Utilities|Array|MakeArray _array_index _array_index_2))
          (LocalVariables|SetNewCurrentUnit _array_element_2)))
      (return (* (Utilities|Array|Get(acopy) (Utilities|Select :Index (Utilities|Array|Get(acopy) (LocalVariables|GetSelectedUnits)) :Option%200 (LocalVariables|GetCm) :Option%201 (LocalVariables|GetMeters) :Option%202 (LocalVariables|GetKm) :Option%203 (LocalVariables|GetInch) :Option%204 (LocalVariables|GetFoot) :Option%205 (LocalVariables|GetYard) :Option%206 (LocalVariables|GetMiles)) (Utilities|Array|Get(acopy) (LocalVariables|GetSelectedUnits) 1)) Distance) (LocalVariables|GetNewCurrentUnit)))))

(fn ConvertLocationbyUnit
  (params (CurrentLocationUnit :type Enum_Distance%20Enum :default "NewEnumerator0") (NewLocationUnit :type Enum_Distance%20Enum :default "NewEnumerator0") (Location :type Vector))
  (bind (_array_element _array_index) (Utilities|Array|ForEachLoopwithBreak (LocalVariables|GetUnit) :!label _label)
    (:LoopBody
      (if (== _array_element CurrentLocationUnit)
        (goto _label Break)))
    (:Completed
      (for (_array_element_2 _array_index_2) (LocalVariables|GetUnit)
        (if (== _array_element_2 NewLocationUnit)
          (LocalVariables|SetSelectedUnits (Utilities|Array|MakeArray _array_index _array_index_2))
          (LocalVariables|SetNewCurrentUnit _array_element_2)))
      (return (* Location (Utilities|Array|Get(acopy) (Utilities|Select :Index (Utilities|Array|Get(acopy) (LocalVariables|GetSelectedUnits)) :Option%200 (LocalVariables|GetCm) :Option%201 (LocalVariables|GetMeters) :Option%202 (LocalVariables|GetKm) :Option%203 (LocalVariables|GetMiles)) (Utilities|Array|Get(acopy) (LocalVariables|GetSelectedUnits) 1))) (LocalVariables|GetNewCurrentUnit)))))