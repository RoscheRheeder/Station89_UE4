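; Actor Blueprint that lays out a configurable 2D grid of one static mesh.
; The Construction Script adds X times Y Hierarchical Instanced Static Mesh instances, deriving row and column from a flat index and spacing them by SpaceX and SpaceY.
; It assigns the mesh inside the loop after each added instance.
; The Z variable is unused, and the Event Graph holds only disabled placeholder events.
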(event EventBeginPlay)

(event Collision|EventActorBeginOverlap
  (params (OtherActor :type Actor%20Object%20Reference)))

(event EventTick
  (params (DeltaSeconds :type Float%20%28single-precision%29)))

(fn ConstructionScript
  (bind _y (Variables|Default|GetY))
  (bind _hierarchicalinstancedstaticmesh (Variables|Default|GetHierarchicalInstancedStaticMesh))
  ;[1 1 1] Array 2D
  (for _index (range 0 (- (* (Variables|Default|GetX) (Variables|Default|GetY)) 1))
    (Components|InstancedStaticMesh|AddInstance _hierarchicalinstancedstaticmesh (Math|Transform|MakeTransform (Math|Vector|MakeVector (* (/ _index _y) (Variables|Default|GetSpace_X)) (* (Math|Integer|%(Integer) _index _y) (Variables|Default|GetSpace_Y)) 0.0)))
    (Components|StaticMesh|SetStaticMesh _hierarchicalinstancedstaticmesh (Variables|Default|GetStatic%20Mesh))))