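; Electrical pole prop that strings three cable components to the pole set in NextElectricalPole, forming power lines in the level.
; The construction script converts that pole's three sphere positions into this actor's local space as cable end points, or destroys the cables when no next pole is valid.
; Slack comes from cable gravity scale, either randomized or set per cable.
; ResetWire has no effect, and the event graph is empty.
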(event EventBeginPlay)

(event Collision|EventActorBeginOverlap
  (params (OtherActor :type Actor%20Object%20Reference)))

(event EventTick
  (params (DeltaSeconds :type Float%20%28single-precision%29)))

(fn ConstructionScript
  ;[1 1 1] Cable 1
  (if (Variables|Default|GetResetWire)
    _
    (else
      _))
  (Utilities|IsValid (Variables|Default|GetNextElectricalPole)
    (:Is%20Valid
      (Variables|/Script/CableComponent.CableComponent|SetEndLocation (Variables|Default|GetCable1) (Math|Transform|InverseTransformLocation (Transformation|GetActorTransform) (Transformation|GetWorldLocation (Variables|BP_ElectricalPole_C|GetSphere1 (Variables|Default|GetNextElectricalPole)))))
      ;[1 1 1] Cable 2
      (Variables|/Script/CableComponent.CableComponent|SetEndLocation (Variables|Default|GetCable2) (Math|Transform|InverseTransformLocation (Transformation|GetActorTransform) (Transformation|GetWorldLocation (Variables|Default|GetSphere2 (Variables|Default|GetNextElectricalPole)))))
      ;[1 1 1] Cable 3
      (Variables|/Script/CableComponent.CableComponent|SetEndLocation (Variables|Default|GetCable3) (Math|Transform|InverseTransformLocation (Transformation|GetActorTransform) (Transformation|GetWorldLocation (Variables|Default|GetSphere3 (Variables|Default|GetNextElectricalPole)))))
      ;[1 1 1] Cable Slack
      (if (Variables|Default|GetIsRandomHang)
        ;;[1 1 1] Randomized Cable Slack
        (Variables|/Script/CableComponent.CableComponent|SetCableGravityScale (Variables|Default|GetCable1) (Math|Random|RandomFloatinRange 1.0 1e+01))
        (Variables|/Script/CableComponent.CableComponent|SetCableGravityScale (Variables|Default|GetCable2) (Math|Random|RandomFloatinRange 1.0 1e+01))
        (Variables|/Script/CableComponent.CableComponent|SetCableGravityScale (Variables|Default|GetCable3) (Math|Random|RandomFloatinRange 1.0 1e+01))
        (else
          ;;[1 1 1] Non-Randomized Cable Slack
          (Variables|/Script/CableComponent.CableComponent|SetCableGravityScale (Variables|Default|GetCable1) (Variables|Default|GetCable1Hang))
          (Variables|/Script/CableComponent.CableComponent|SetCableGravityScale (Variables|Default|GetCable2) (Variables|Default|GetCable2Hang))
          (Variables|/Script/CableComponent.CableComponent|SetCableGravityScale (Variables|Default|GetCable3) (Variables|Default|GetCable3Hang)))))
    (:Is%20Not%20Valid
      (Components|DestroyComponent (Variables|Default|GetCable1)))))