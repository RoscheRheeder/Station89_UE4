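; BP_EQController is an audio visualizer that plays a track and animates a grid of spawned BP_AudioCube actors as an equalizer.
; BeginPlay starts the audio and builds the grid, optionally shuffling the cube array so frequency bands look less linear.
; Each Tick samples the track's frequency spectrum at current game time, one band per cube.
; Band magnitude drives either cube height or Z scale, chosen by flags.
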(event EventBeginPlay
  (Audio|Components|Audio|SetSound (Variables|Default|GetAudio) (Variables|Default|GetAudioTrack))
  (Audio|Components|Audio|Play (Variables|Default|GetAudio) 0.0)
  (CallFunction|SpawnGrid)
  (if (Variables|Default|GetRandomCubePosition)
    ;[1 1 1] Make cubes less-linear
    (Utilities|Array|Shuffle (Variables|Default|GetBP_CubeArray))))

(event EventTick
  (params (DeltaSeconds :type Float%20%28single-precision%29))
  (bind _outspectrum (Class|SoundVisualizationStatics|CalculateFrequencySpectrum (Variables|Default|GetAudioTrack) 0 (Utilities|Time|GetGameTimeinSeconds) 0.1 (Utilities|Array|Length (Variables|Default|GetBP_CubeArray))))
  (Variables|Default|SetSpectrum _outspectrum)
  (for (_array_element _array_index) (Variables|Default|GetBP_CubeArray)
    (if (Variables|Default|GetUseLocation)
      (Transformation|SetActorLocation _array_element (Math|Vector|MakeVector (.x (Transformation|GetActorLocation _array_element)) (.y (Transformation|GetActorLocation _array_element)) (Math|Float|NormalizetoRange (* (Math|Float|Absolute(Float) (Utilities|Array|Get(acopy) (Variables|Default|GetSpectrum) _array_index)) 1e+01) 0.0 1.0)) false false)
      (elif (Variables|Default|GetUseScale)
        (Transformation|SetActorScale3D _array_element (Math|Vector|MakeVector 1.0 1.0 (* (Math|Float|Absolute(Float) (Utilities|Array|Get(acopy) (Variables|Default|GetSpectrum) _array_index)) 0.1)))))))

(fn ConstructionScript)

(fn SpawnGrid
  (bind _distance (Variables|Default|GetDistance))
  (for _index (range 0 (- (Variables|Default|GetNumCubes) 1))
    (bind _returnvalue (Game|SpawnActorfromClass "/Game/Audio/AudioVisualizer/BP_AudioCube.BP_AudioCube_C" (Math|Transform|MakeTransform (Math|Vector|MakeVector (* (Variables|Default|GetRow) _distance) (* (Variables|Default|GetCol) _distance) 0.0) "0, 0, 0" "1,1,1") "AlwaysSpawn" 0 0))
    (Utilities|Array|Add (Variables|Default|GetBP_CubeArray) _returnvalue)
    (Math|Integer|IncrementInt (Variables|Default|GetRow)
      (:%20%20
        (if (== (Variables|Default|GetRow) (Math|Float|Truncate (Math|Float|Sqrt (Math|Conversions|ToFloat(Integer) (Variables|Default|GetNumCubes)))))
          (Math|Integer|IncrementInt (Variables|Default|GetCol)
            (:%20%20
              (Variables|Default|SetRow 0))))))))