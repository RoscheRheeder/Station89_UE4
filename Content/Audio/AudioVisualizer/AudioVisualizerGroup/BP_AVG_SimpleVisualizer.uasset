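; Simple audio visualizer actor that makes every BP_AVG_Sphere in the level pulse with the loudness of its sound.
; It starts its Audio component on BeginPlay and listens to the single envelope value event.
; Each envelope update finds all sphere actors, uniformly scales their meshes by the envelope times a multiplier, and prints the value for debugging.
; The multi-envelope handler is empty.
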(event OnAudioSingleEnvelopeValue(Audio)
  (params (PlayingSoundWave :type Sound%20Wave%20Object%20Reference) (EnvelopeValue :type Float%20%28single-precision%29))
  ;[1 0 0 1 14] TODO: Search up what these are
  (bind _outactors (Actor|GetAllActorsOfClass "/Game/Audio/AudioVisualizer/AudioVisualizerGroup/BP_AVG_Sphere.BP_AVG_Sphere_C"))
  (for _array_element _outactors
    (Transformation|SetRelativeScale3D (Variables|/Game/Audio/AudioVisualizer/AudioVisualizerGroup/BP_AVG_Sphere.BP_AVG_Sphere_C|GetSM_Sphere _array_element) (Math|Conversions|ToVector(Float) (* EnvelopeValue (Variables|Default|GetScaleMultiplier))))
    (Development|PrintString (Utilities|String|Append (Utilities|GetObjectName _array_element) (Utilities|String|ToString(Float) EnvelopeValue)))))

(event OnAudioMultiEnvelopeValue(Audio)
  (params (AverageEnvelopeValue :type Float%20%28single-precision%29) (MaxEnvelope :type Float%20%28single-precision%29) (NumWaveInstances :type Integer))
  ;[1 0 0 1 14] TODO: Search up what these are
)

(event EventBeginPlay
  (Audio|Components|Audio|Play (Variables|Default|GetAudio) 0.0))

(event Collision|EventActorBeginOverlap
  (params (OtherActor :type Actor%20Object%20Reference)))

(event EventTick
  (params (DeltaSeconds :type Float%20%28single-precision%29)))

(fn ConstructionScript)